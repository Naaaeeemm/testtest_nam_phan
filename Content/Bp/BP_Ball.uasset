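; BP_Ball is a ball that the player launches with a charged Space bar press.
; While Space is held, Tick accumulates the hold time.
; On release, it enables physics on the Sphere and applies a vertical impulse scaled by hold time over the maximum charge duration, clamped to full strength.
; The charge then resets for the next press.
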(event `self.ReceiveTick`
  (params (DeltaSeconds :type "Float (single-precision)"))
  (if (`self.IsSpaceBarPressed`)
    (set `self.SpaceBarHeldDuration` (+ DeltaSeconds (`self.SpaceBarHeldDuration`)))))

(event `Key|SpaceBar`
  (params (Key :type "Key Structure"))
  (:`Pressed`
    (set `self.IsSpaceBarPressed` true))
  (:`Released`
    (`PrimitiveComponent.SetSimulatePhysics` (`self.Sphere`) true)
    (`PrimitiveComponent.AddImpulse` (`self.Sphere`) (`KismetMathLibrary.MakeVector` 0.0 0.0 (* (`self.Impulse Strenght`) (`KismetMathLibrary.FClamp` (/ (`self.SpaceBarHeldDuration`) (`self.MaxChargeDuration`)) 0.0 1.0))) "None" false)
    (set `self.IsSpaceBarPressed` false)
    (set `self.SpaceBarHeldDuration` 0.0)))

(fn `UserConstructionScript`)